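; Clickable marker actor that toggles a Monsanto info widget on screen.
; BeginPlay enables the mouse cursor and click events, and a FlipFlop on marker clicks alternately creates the widget in the viewport or removes it.
; Every Tick, the root's world scale is set to the camera-to-marker distance divided by ScaleFactor, keeping the marker's apparent size constant.
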(event OnClicked(MarkerNew)
  (params (TouchedComponent :type Primitive%20Component%20Object%20Reference) (ButtonPressed :type Key%20Structure :default "None"))
  ;[0.1407 0.1494 1] On Click UI POP up
  (Utilities|FlowControl|FlipFlop
    (:A
      (bind _returnvalue (UserInterface|CreateWidget "/Game/UI_Widgets/Ui_Widget_Monsanto.Ui_Widget_Monsanto_C"))
      (bind _output_get (Variables|Default|SetMonsantoWidVar _returnvalue))
      (UserInterface|Viewport|AddtoViewport _output_get 0))
    (:B
      (Widget|RemovefromParent (Variables|Default|GetMonsantoWidVar)))))

(event EventBeginPlay
  ;[1 0.04161 0.05156] Enable Clicking/Mouse Cursor
  (Variables|/Script/Engine.PlayerController|SetbEnableClickEvents (Game|GetPlayerController 0) true)
  (Variables|/Script/Engine.PlayerController|SetbShowMouseCursor (Game|GetPlayerController 0) true))

(event EventTick
  (params (DeltaSeconds :type Float%20%28single-precision%29))
  ;[0.9616 1 0.09615] Scaling
  (Transformation|SetWorldScale3D (Variables|Default|GetDefaultSceneRoot) (Math|Conversions|ToVector(Float) (Math|Float|SafeDivide (Math|Vector|VectorLength (- (Camera|GetCameraLocation (Game|GetPlayerCameraManager 0)) (Transformation|GetWorldLocation (Variables|Default|GetMarkerNew)))) (Variables|Default|GetScaleFactor)))))

(fn ConstructionScript)