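; BP_Eduardo7 is an actor with a clickable MarkerNew component that opens and closes a UI pop-up.
; Clicking the marker runs a FlipFlop that alternates between creating a Ui_Widget_Eduardo7 widget and adding it to the viewport, and removing it.
; A fresh widget is created on each opening and stored in a variable for the later removal.
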(event OnClicked(MarkerNew)
  (params (TouchedComponent :type Primitive%20Component%20Object%20Reference) (ButtonPressed :type Key%20Structure :default "None"))
  ;[0.1407 0.1494 1] On Click UI POP up
  (Utilities|FlowControl|Sequence
    (:then_1
      (Utilities|FlowControl|FlipFlop
        (:A
          (bind _returnvalue (UserInterface|CreateWidget "/Game/UI_Widgets/Ui_Widget_Eduardo7.Ui_Widget_Eduardo7_C"))
          (bind _output_get (Variables|Default|SetNewVar _returnvalue))
          (UserInterface|Viewport|AddtoViewport _output_get 0))
        (:B
          (Widget|RemovefromParent (Variables|Default|GetNewVar)))))))

(event EventBeginPlay
  (|CallParentFunction) ; This node is disabled and will not be called.\nDrag off pins to build functionality.
)

(event Collision|EventActorBeginOverlap
  (params (OtherActor :type Actor%20Object%20Reference)))

(event EventTick
  (params (DeltaSeconds :type Float%20%28single-precision%29))
  (|CallParentFunction DeltaSeconds) ; This node is disabled and will not be called.\nDrag off pins to build functionality.
)

(fn ConstructionScript
  (|CallParentFunction))