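; BP_BaseMarker is a base marker actor that adjusts its scale to the player camera's distance.
; On BeginPlay it enables click events and shows the mouse cursor on the first player controller.
; Every Tick it sets the root's uniform world scale to the camera-to-MarkerNew distance divided by ScaleFactor, so its apparent on-screen size stays roughly constant.
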(event EventBeginPlay
  ;[1 0.04161 0.05156] Enable Clicking/Mouse Cursor
  (Variables|/Script/Engine.PlayerController|SetbEnableClickEvents (Game|GetPlayerController 0) true)
  (Variables|/Script/Engine.PlayerController|SetbShowMouseCursor (Game|GetPlayerController 0) true))

(event EventTick
  (params (DeltaSeconds :type Float%20%28single-precision%29))
  ;[0.9616 1 0.09615] Scaling
  (Transformation|SetWorldScale3D (Variables|Default|GetDefaultSceneRoot) (Math|Conversions|ToVector(Float) (Math|Float|SafeDivide (Math|Vector|VectorLength (- (Camera|GetCameraLocation (Game|GetPlayerCameraManager 0)) (Transformation|GetWorldLocation (Variables|Default|GetMarkerNew)))) (Variables|Default|GetScaleFactor)))))

(fn ConstructionScript)